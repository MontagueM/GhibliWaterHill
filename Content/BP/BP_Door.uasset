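; Door Blueprint for VR that swings when a controller grabs its handle.
; The Grabbed event checks that the grabbed component is HandleMesh, then sets DoorMesh's relative yaw from the controller's world yaw, clamped between -90 and 90 degrees.
; Roll and pitch are preserved, and the rotation is applied only when Grabbed fires, with no sweep.
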(event `Grabbed`
  (params (VRController :type "VRController Object Reference") (GrabbedComponent :type "PrimitiveComponent Object Reference"))
  (bind _door_mesh (`self.Door Mesh`))
  (if (== GrabbedComponent (`self.Handle Mesh`))
    (`SceneComponent.K2_SetRelativeRotation` _door_mesh (`KismetMathLibrary.MakeRotator` (.roll (`SceneComponent.RelativeRotation` _door_mesh)) (.pitch (`SceneComponent.RelativeRotation` _door_mesh)) (`KismetMathLibrary.FClamp` (.yaw (`self.K2_GetActorRotation` VRController)) -90.0 90.0)) false false)))

(fn `UserConstructionScript`)